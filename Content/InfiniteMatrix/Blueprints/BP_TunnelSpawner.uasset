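; Spawner actor that builds an endless-style chain of BP_Tunnel segments, starting at the player pawn on BeginPlay.
; Startup clears existing tunnels, spawns a few linked segments, then removes all health packs and enemies.
; Each new segment attaches at the newest one's SpawnPoint, gets a spawner back-reference and randomized wall, and may spawn randomly offset extra actors.
; A running count switches later segments to blue materials.
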(event EventBeginPlay
  (CallFunction|SpawnInitialTunnels))

(event Collision|EventActorBeginOverlap
  (params (OtherActor :type Actor%20Object%20Reference)))

(event EventTick
  (params (DeltaSeconds :type Float%20%28single-precision%29)))

(fn ConstructionScript)

(fn SpawnTunnel
  (params (SpawnLocationX :type Float%20%28double-precision%29) (SpawnLocationY :type Float%20%28double-precision%29) (SpawnLocationZ :type Float%20%28double-precision%29))
  (bind _returnvalue (Game|SpawnActorfromClass "/Game/InfiniteMatrix/Blueprints/BP_Tunnel.BP_Tunnel_C" (Math|Transform|MakeTransform (Math|Vector|MakeVector SpawnLocationX SpawnLocationY SpawnLocationZ) "0, 0, 0" "1.000000,1.000000,1.000000") "Undefined" "MultiplyWithRoot" 0 0))
  (Variables|Default|SetNum (+ (Variables|Default|GetNum) 1.0))
  (if (>= (+ (Variables|Default|GetNum) 1.0) 1e+01)
    (Utilities|IsValid _returnvalue
      (:Is%20Valid
        (Rendering|Material|SetMaterial (Variables|/Script/Engine.StaticMeshActor|GetStaticMeshComponent _returnvalue) 0 "/Game/InfiniteMatrix/Materials/Blue_Tunnel.Blue_Tunnel")
        (Rendering|Material|SetMaterial (Variables|/Game/InfiniteMatrix/Blueprints/BP_Tunnel.BP_Tunnel_C|GetWallMesh _returnvalue) 0 "/Game/InfiniteMatrix/Materials/Blue_hole.Blue_hole"))))
  (bind _output_get (Variables|Default|SetNewestTunnel _returnvalue))
  (Variables|/Game/InfiniteMatrix/Blueprints/BP_Tunnel.BP_Tunnel_C|SetTunnelSpawner _output_get self)
  (Default|RandomizeWall _output_get)
  (if (> (Math|Random|RandomFloatinRange 0.0 1e+02) 5e+01)
    (Game|SpawnActorfromClass "/Game/InfiniteMatrix/Blueprints/BP_HealthPack.BP_HealthPack_C" (Math|Transform|MakeTransform (Math|Vector|MakeVector (+ SpawnLocationX (Math|Random|RandomFloatinRange 8e+02 1.8e+03)) (+ SpawnLocationY (Math|Random|RandomFloatinRange -2e+02 2e+02)) (+ SpawnLocationZ (Math|Random|RandomFloatinRange -2e+02 2e+02))) "0.000000,90.000000,0.000000" "1.500000,1.500000,1.500000") "Undefined" "MultiplyWithRoot" 0 0))
  (if (> (Math|Random|RandomFloatinRange 0.0 1e+02) 3e+01)
    (Game|SpawnActorfromClass "/Game/InfiniteMatrix/Blueprints/BP_Enemy.BP_Enemy_C" (Math|Transform|MakeTransform (Math|Vector|MakeVector (+ SpawnLocationX (Math|Random|RandomFloatinRange 8e+02 1.8e+03)) (+ SpawnLocationY (Math|Random|RandomFloatinRange -2e+02 2e+02)) (+ SpawnLocationZ (Math|Random|RandomFloatinRange -2e+02 2e+02))) "0, 0, 0" "1.000000,1.000000,1.000000") "Undefined" "MultiplyWithRoot" 0 0)))

(fn SpawnTunnelatSpawnPoint
  (bind _newesttunnel (Variables|Default|GetNewestTunnel))
  (bind _spawnpoint (Variables|/Game/InfiniteMatrix/Blueprints/BP_Tunnel.BP_Tunnel_C|GetSpawnPoint _newesttunnel))
  (bind _returnvalue (Transformation|GetWorldLocation _spawnpoint))
  (bind (_x _y _z) (Math|Vector|BreakVector _returnvalue))
  (CallFunction|SpawnTunnel _x _y _z))

(fn SpawnInitialTunnels
  (bind _returnvalue (Game|Player|GetPlayerPawn 0))
  (bind _returnvalue_2 (Transformation|GetActorLocation _returnvalue))
  (bind (_x _y _z) (Math|Vector|BreakVector _returnvalue_2))
  (Utilities|FlowControl|Sequence
    (:then_0
      (bind _outactors (Actor|GetAllActorsOfClass "/Game/InfiniteMatrix/Blueprints/BP_Tunnel.BP_Tunnel_C"))
      (for _array_element _outactors
        (Actor|DestroyActor _array_element)))
    (:then_1
      (for _index (range 0 2)
        (Utilities|IsValid (Variables|Default|GetNewestTunnel)
          (:Is%20Valid
            (CallFunction|SpawnTunnelatSpawnPoint))
          (:Is%20Not%20Valid
            (CallFunction|SpawnTunnel _x _y _z)))))
    (:then_2
      (bind _outactors_2 (Actor|GetAllActorsOfClass "/Game/InfiniteMatrix/Blueprints/BP_HealthPack.BP_HealthPack_C"))
      (for _array_element_2 _outactors_2
        (Actor|DestroyActor _array_element_2)))
    (:then_3
      (bind _outactors_3 (Actor|GetAllActorsOfClass "/Game/InfiniteMatrix/Blueprints/BP_Enemy.BP_Enemy_C"))
      (for _array_element_3 _outactors_3
        (Actor|DestroyActor _array_element_3)))))